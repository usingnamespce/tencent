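; Test bullet projectile that explodes on hitting a "CanDamaged"-tagged actor or when its speed drops to 500 or below.
; Tick checks speed behind a half-second Delay, and both triggers feed shared explosion effect and sound logic through DoOnce gates.
; Authority damages the last hit actor, crediting the owning BP_Character's controller, and destroys the bullet only if that actor can be damaged.
; Remote instances simply hide and destroy it.
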(event EventBeginPlay)

(event Collision|EventHit
  (params (MyComp :type Primitive%20Component%20Object%20Reference) (Other :type Actor%20Object%20Reference) (OtherComp :type Primitive%20Component%20Object%20Reference) (bSelfMoved :type Boolean) (HitLocation :type Vector :default "0, 0, 0") (HitNormal :type Vector :default "0, 0, 0") (NormalImpulse :type Vector :default "0, 0, 0") (Hit :type Hit%20Result%20Structure%20%28by%20ref%29))
  (bind _returnvalue (Transformation|GetActorLocation))
  (Variables|Default|SetOther Other)
  (if (Actor|ActorHasTag Other "CanDamaged")
    (Utilities|FlowControl|DoOnce false
      (:Completed
        (Effects|SpawnEmitteratLocation "/Game/FX/Particles/P_Explosion.P_Explosion" _returnvalue)
        (Audio|PlaySoundatLocation "/Game/Audio/Explosion01.Explosion01" _returnvalue "0, 0, 0" 1.0 1.0 0.0 0 0 0)
        (Networking|SwitchHasAuthority
          (:Authority
            (if (Variables|/Script/Engine.Actor|GetbCanBeDamaged (Variables|Default|GetOther))
              (Game|Damage|ApplyDamage (Variables|Default|GetOther) 2e+01 (Pawn|GetController (.AsBP%20Character (Utilities|Casting|CastToBP_Character (Components|GetOwner)))) 0)
              (Rendering|SetActorHiddenInGame true)
              (Actor|DestroyActor)))
          (:Remote
            (Rendering|SetActorHiddenInGame true)
            (Actor|DestroyActor)))))))

(event EventTick
  (params (DeltaSeconds :type Float%20%28single-precision%29))
  (bind _returnvalue (Transformation|GetActorLocation))
  (Utilities|FlowControl|Delay 0.5)
  (if (<= (Math|Vector|VectorLength (Transformation|GetVelocity)) 5e+02)
    (Utilities|FlowControl|DoOnce false
      (:Completed
        (Effects|SpawnEmitteratLocation "/Game/FX/Particles/P_Explosion.P_Explosion" _returnvalue)
        (Audio|PlaySoundatLocation "/Game/Audio/Explosion01.Explosion01" _returnvalue "0, 0, 0" 1.0 1.0 0.0 0 0 0)
        (Networking|SwitchHasAuthority
          (:Authority
            (if (Variables|/Script/Engine.Actor|GetbCanBeDamaged (Variables|Default|GetOther))
              (Game|Damage|ApplyDamage (Variables|Default|GetOther) 2e+01 (Pawn|GetController (.AsBP%20Character (Utilities|Casting|CastToBP_Character (Components|GetOwner)))) 0)
              (Rendering|SetActorHiddenInGame true)
              (Actor|DestroyActor)))
          (:Remote
            (Rendering|SetActorHiddenInGame true)
            (Actor|DestroyActor)))))))

(fn ConstructionScript)