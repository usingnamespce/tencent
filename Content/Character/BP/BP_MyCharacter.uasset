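; Player character Blueprint handling movement stances, gun and sword combat, item pickup and footprints.
; Timelines ramp sprint speed and camera boom height for gun-only crouch and prone toggles, which are throttled by DoOnce and delays.
; A weapon-struct array tracks socket-attached guns, swapped with the sword through visibility.
; BeginPlay creates the HUD and starts a looping camera trace that highlights BP_Props for pickup, while FootprintComponent spawns decals for key-cycled footwear.
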(event Custom|OpenCrouch
  (bind _returnvalue (Pawn|GetController))
  ;[1 1 1] Crouch
  (Utilities|FlowControl|DoOnce false) ; enters at Reset
)

(event Custom|OpenProne
  ;[1 1 1] Prone
  (Utilities|FlowControl|DoOnce false) ; enters at Reset
)

(event Input|ActionEvents|InputActionSprint
  (params (Key :type Key%20Structure :default "None"))
  ;[1 1 1] Sprint
  (:Pressed
    (bind _speed (Timeline|SprintBuffer PlayFromStart)
      (:Update
        (Variables|/Script/Engine.CharacterMovementComponent|SetMaxWalkSpeed (Variables|Character|GetCharacterMovement) _speed))))
  (:Released
    (Timeline|SprintBuffer ReverseFromEnd)))

(event Input|ActionEvents|InputActionCrouch
  (params (Key :type Key%20Structure :default "None"))
  (bind _returnvalue (Pawn|GetController))
  ;[1 1 1] Crouch
  (:Pressed
    (if (Utilities|IsUseGun)
      (Utilities|FlowControl|DoOnce false
        (:Completed
          (Utilities|FlowControl|Sequence
            (:then_0
              (if (Utilities|Enum|NotEqual(Enum) (Variables|Default|GetAniState) "NewEnumerator2")
                (Utilities|FlowControl|FlipFlop
                  (:A
                    (Character|Crouch)
                    (Variables|Default|SetAniState "NewEnumerator1")
                    (Input|SetIgnoreMoveInput _returnvalue true)
                    (bind _hight (Timeline|CameraBufferCourch ReverseFromEnd)
                      (:Update
                        (Transformation|SetRelativeLocation (Variables|Default|GetCameraBoom) (Math|Vector|MakeVector 0.0 7e+01 _hight) false false))
                      (:Finished
                        (Input|SetIgnoreMoveInput (Pawn|GetController) false))))
                  (:B
                    (Character|UnCrouch)
                    (Variables|Default|SetAniState "NewEnumerator0")
                    (Input|SetIgnoreMoveInput _returnvalue true)
                    (Timeline|CameraBufferCourch PlayFromStart)))))
            (:then_1
              (Utilities|FlowControl|Delay 1.0)
              (CallFunction|OpenCrouch))))))))

(event Input|ActionEvents|InputActionProne
  (params (Key :type Key%20Structure :default "None"))
  ;[1 1 1] Prone
  (:Pressed
    (if (Utilities|IsUseGun)
      (Utilities|FlowControl|DoOnce false
        (:Completed
          (Utilities|FlowControl|Sequence
            (:then_0
              (if (Utilities|Enum|NotEqual(Enum) (Variables|Default|GetAniState) "NewEnumerator1")
                (Utilities|FlowControl|FlipFlop
                  (:A
                    (Variables|Default|SetAniState "NewEnumerator2")
                    (Input|SetIgnoreMoveInput (Pawn|GetController) true)
                    (Variables|/Script/Engine.CharacterMovementComponent|SetJumpZVelocity (Variables|Character|GetCharacterMovement) 0.0)
                    (bind _hight (Timeline|CameraBufferProne ReverseFromEnd)
                      (:Update
                        (Transformation|SetRelativeLocation (Variables|Default|GetCameraBoom) (Math|Vector|MakeVector 0.0 7e+01 _hight) false false))
                      (:Finished
                        (if (Utilities|Enum|Equal(Enum) (Variables|Default|GetAniState) "NewEnumerator0")
                          (Input|SetIgnoreMoveInput (Pawn|GetController) false)
                          (Variables|/Script/Engine.CharacterMovementComponent|SetJumpZVelocity (Variables|Character|GetCharacterMovement) 6e+02)))))
                  (:B
                    (Variables|Default|SetAniState "NewEnumerator0")
                    (Timeline|CameraBufferProne PlayFromStart)))))
            (:then_1
              (Utilities|FlowControl|Delay 1.0)
              (CallFunction|OpenProne))))))))

(event Input|ActionEvents|InputActionFreeView
  (params (Key :type Key%20Structure :default "None"))
  (bind _charactermovement (Variables|Character|GetCharacterMovement))
  ;[1 1 1] FreeView
  (:Pressed
    (Variables|/Script/Engine.CharacterMovementComponent|SetbUseControllerDesiredRotation _charactermovement false))
  (:Released
    (Variables|/Script/Engine.CharacterMovementComponent|SetbUseControllerDesiredRotation _charactermovement true)))

(event Input|ActionEvents|InputActionFire
  (params (Key :type Key%20Structure :default "None"))
  (bind _usingweapon (Variables|Default|GetUsingWeapon))
  (bind _weaponref (Utilities|Struct|BreakStruct_WeaponState _usingweapon))
  ;[1 1 1] Fire
  (:Pressed
    (if (Utilities|IsUseGun)
      (if (Variables|Default|GetbCanFire)
        (Variables|Default|SetbCanFire false)
        (Default|Fire _weaponref)
        (Utilities|FlowControl|Delay (Variables|/Game/BP/Props/Gun/BP_Props_Gun.BP_Props_Gun_C|GetFireTime _weaponref))
        (Variables|Default|SetbCanFire true)))))

(event Input|ActionEvents|InputActionChangeWeapon
  (params (Key :type Key%20Structure :default "None"))
  ;[1 1 1] ChangeWeapon
  (:Pressed
    (if (Utilities|Array|IsValidIndex (Variables|Default|GetWeaponState))
      (Animation|Montage|MontageStop (Components|SkeletalMesh|GetAnimInstance (Variables|Character|GetMesh)) 0.0 0)
      (Utilities|FlowControl|FlipFlop
        (:A
          (CallFunction|ChangeGun "NewEnumerator0")
          (Rendering|SetActorHiddenInGame (.WeaponRef (Utilities|Struct|BreakStruct_WeaponState (Variables|Default|GetUsingWeapon))) false)
          (Rendering|SetVisibility (Variables|Default|GetSword) false false))
        (:B
          (Variables|Default|SetUsingWeapon (Utilities|Struct|MakeStruct_WeaponState "NewEnumerator1" (.SocketName (Utilities|Struct|BreakStruct_WeaponState (Variables|Default|GetUsingWeapon))) (.WeaponRef (Utilities|Struct|BreakStruct_WeaponState (Variables|Default|GetUsingWeapon)))))
          (Rendering|SetActorHiddenInGame (.WeaponRef (Utilities|Struct|BreakStruct_WeaponState (Variables|Default|GetUsingWeapon))) true)
          (Rendering|SetVisibility (Variables|Default|GetSword) true false))))))

(event Input|ActionEvents|InputActionSwordAttack
  (params (Key :type Key%20Structure :default "None"))
  ;[1 1 1] SwordAttack
  (:Pressed
    (if (not (Utilities|IsUseGun))
      (Animation|Montage|PlayMontage (Variables|Character|GetMesh) "/Game/Character/Animations/Montage/Twinblades_attack02_Montage.Twinblades_attack02_Montage"))))

(event Custom|LineTrack
  (bind _followcamera (Variables|Default|GetFollowCamera))
  (bind _returnvalue (Transformation|GetWorldLocation _followcamera))
  (bind _outhit (Collision|LineTraceByChannel _returnvalue (+ _returnvalue (* (Math|Vector|GetForwardVector (Transformation|GetWorldRotation _followcamera)) 4e+02)) "TraceTypeQuery3" false 0 "None"))
  (if (.bBlockingHit (Collision|BreakHitResult _outhit))
    (bind _asbp_props (Utilities|Casting|CastToBP_Props (.HitActor (Collision|BreakHitResult _outhit))))
    (bind _output_get (Variables|Default|SetHitActor _asbp_props))
    (Default|RenderBegin _output_get)
    (else
      (Utilities|IsValid (Variables|Default|GetHitActor)
        (:Is%20Valid
          (Default|RenderEnd (Variables|Default|GetHitActor))
          (Variables|Default|SetHitActor 0))))))

(event EventBeginPlay
  (bind _returnvalue (UserInterface|CreateWidget "/Game/BP/Widget/Wid_HUD.Wid_HUD_C"))
  (UserInterface|Viewport|AddtoViewport _returnvalue 0)
  (Variables|/Game/footprint/Blueprints/FootprintComponent.FootprintComponent_C|SetMesh (Variables|Default|GetFootprintComponent) (Variables|Character|GetMesh))
  (Variables|/Game/footprint/Blueprints/FootprintComponent.FootprintComponent_C|SetCurrentFootwear (Variables|Default|GetFootprintComponent) (Variables|Default|GetCurrentFootwear))
  (Utilities|Time|SetTimerbyEvent (delegate Custom|LineTrack) 0.1 true))

(event EventChangeFootState
  (params (New%20Style :type EFootState%20Enum :default "NewEnumerator0"))
  (Variables|/Game/footprint/Blueprints/FootprintComponent.FootprintComponent_C|SetFootState (Variables|Default|GetFootprintComponent) New%20Style))

(event EventSpawnDecal
  (params (SocketName :type Name :default "None") (Right :type Boolean) (Left :type Boolean))
  (Default|SpawnDecal (Variables|Default|GetFootprintComponent) SocketName Right Left))

(event Input|ActionEvents|InputActionPickUp
  (params (Key :type Key%20Structure :default "None"))
  (bind _hitactor (Variables|Default|GetHitActor))
  (:Pressed
    (Utilities|IsValid _hitactor
      (:Is%20Valid
        (Class|BPIProps|PickUp(Message) _hitactor)))))

(event Input|KeyboardEvents|E
  (params (Key :type Key%20Structure :default "None"))
  ;[1 1 1] Switching between Footwear
  (:Pressed
    (switch Utilities|FlowControl|Switch|SwitchonEFootprintStyle (Variables|Default|GetCurrentFootwear)
      (:NewEnumerator0
        (Variables|Default|SetCurrentFootwear "NewEnumerator1"))
      (:NewEnumerator1
        (Variables|Default|SetCurrentFootwear "NewEnumerator6"))
      (:NewEnumerator6
        (Variables|Default|SetCurrentFootwear "NewEnumerator3"))
      (:NewEnumerator3
        (Variables|Default|SetCurrentFootwear "NewEnumerator4"))
      (:NewEnumerator4
        (Variables|Default|SetCurrentFootwear "NewEnumerator5"))
      (:NewEnumerator5
        (Variables|Default|SetCurrentFootwear "NewEnumerator0")))
    (bind _output_get (Variables|/Game/footprint/Blueprints/FootprintComponent.FootprintComponent_C|SetCurrentFootwear (Variables|Default|GetFootprintComponent) (Variables|Default|GetCurrentFootwear)))
    (Development|PrintString (Utilities|String|EnumtoString _output_get))))

(event Custom|AddGun
  (params (Weapon :type Enum_Weapon%20Enum :default "NewEnumerator0") (SocketName :type String) (WeaponRef :type BP%20Props%20Gun%20Object%20Reference%20%28by%20ref%29))
  ;[1 1 1] Add
  (Utilities|Array|AddUnique (Variables|Default|GetWeaponState) (Utilities|Struct|MakeStruct_WeaponState Weapon SocketName WeaponRef))
  (Transformation|AttachComponentToComponent WeaponRef (Variables|Character|GetMesh) (Utilities|String|StringToName SocketName) "SnapToTarget" "SnapToTarget" "SnapToTarget" true)
  (Rendering|SetActorHiddenInGame WeaponRef true))

(event Custom|RemoveGun
  (params (Weapon :type Enum_Weapon%20Enum :default "NewEnumerator0"))
  ;[1 1 1] Remove
  (bind (_array_element _array_index) (Utilities|Array|ForEachLoopwithBreak (Variables|Default|GetWeaponState))
    (:LoopBody
      (if (Utilities|Enum|Equal(Enum) (.Weapon (Utilities|Struct|BreakStruct_WeaponState _array_element)) Weapon)
        (Utilities|Array|RemoveIndex (Variables|Default|GetWeaponState) _array_index)
        (if (Utilities|Enum|Equal(Enum) (.Weapon (Utilities|Struct|BreakStruct_WeaponState (Variables|Default|GetUsingWeapon))) (.Weapon (Utilities|Struct|BreakStruct_WeaponState _array_element)))
          (CallFunction|ChangeGun "NewEnumerator1"))))))

(event Custom|ChangeGun
  (params (Weapon :type Enum_Weapon%20Enum :default "NewEnumerator0"))
  ;[1 1 1] Change
  (Utilities|IsValid (.WeaponRef (Utilities|Struct|BreakStruct_WeaponState (Variables|Default|GetUsingWeapon)))
    (:Is%20Valid
      (Rendering|SetActorHiddenInGame (.WeaponRef (Utilities|Struct|BreakStruct_WeaponState (Variables|Default|GetUsingWeapon))) true))
    (:Is%20Not%20Valid
      _))
  (bind (_array_element _array_index) (Utilities|Array|ForEachLoopwithBreak (Variables|Default|GetWeaponState))
    (:LoopBody
      (if (Utilities|Enum|Equal(Enum) (.Weapon (Utilities|Struct|BreakStruct_WeaponState _array_element)) Weapon)
        (bind _output_get (Variables|Default|SetUsingWeapon (Utilities|Array|Get(acopy) (Variables|Default|GetWeaponState) _array_index)))
        (Rendering|SetActorHiddenInGame (.WeaponRef (Utilities|Struct|BreakStruct_WeaponState _output_get)) false)))))

(fn ConstructionScript)