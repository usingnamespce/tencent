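; BP_MyPlayerState is a player state that tracks a player's health, score, kill and death counts, and user name.
; UpdateState subtracts damage unless already dead; at zero health it calls Death on the BP_Character pawn and increments the death count.
; It then awards score and a SkillNum increment to the attacker's player state.
; SetNameClient copies the user name from the game instance for locally controlled pawns.
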(event Custom|SetName
  (params (UserName :type Text))
  (Variables|Default|SetUserName UserName))

(event Custom|UpdateScore
  (params (AddScore :type Integer))
  (Variables|Default|SetPlayerScore (+ (Variables|Default|GetPlayerScore) AddScore))
  (Math|Integer|IncrementInt (Variables|Default|GetSkillNum)))

(event Custom|SetNameClient
  (if (Pawn|IsLocallyControlled (Variables|Default|GetPawnPrivate))
    (CallFunction|SetName (Variables|/Game/BP/Gameplay/BP_MyGameinstance.BP_MyGameinstance_C|GetuserName (.AsBP%20My%20Gameinstance (Utilities|Casting|CastToBP_MyGameinstance (Game|GetGameInstance)))))))

(event Custom|UpdateDealth
  (Math|Integer|IncrementInt (Variables|Default|GetDeathNum)))

(event Custom|UpdateState
  (params (MinusHealth :type Float%20%28single-precision%29) (EnemyState :type BP%20My%20Player%20State%20Object%20Reference) (AddScore :type Integer))
  (if (not (Variables|Default|GetisDeath))
    (bind _output_get (Variables|Default|SetHealth (- (Variables|Default|GetHealth) MinusHealth)))
    (if (<= _output_get 0.0)
      (Variables|Default|SetisDeath true)
      (bind _asbp_character (Utilities|Casting|CastToBP_Character (Variables|Default|GetPawnPrivate)))
      (Default|Death _asbp_character)
      (CallFunction|UpdateDealth)
      (Utilities|IsValid EnemyState
        (:Is%20Valid
          (CallFunction|UpdateScore EnemyState AddScore))))))

(fn ConstructionScript)