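; Rifle ammo pickup prop that adds bullets to a rifle the player carries.
; On pickup it searches the player's WeaponState entries for a BP_Props_Gun_Rifle, raises its BulletNum by AddBulletNum, then destroys itself and ends the loop.
; RenderBegin and RenderEnd toggle custom depth rendering on RampStaticMesh.
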(event EventBeginPlay
  (|CallParentFunction) ; 此节点被禁用，将不会被调用。\n从引脚连出引线来编译功能。
)

(event EventPickUp
  (params (Player :type BP%20Character%20Object%20Reference))
  (bind _array_element (Utilities|Array|ForEachLoopwithBreak (Variables|/Game/Character/BP/BP_Character.BP_Character_C|GetWeaponState Player) :!label _label)
    (:LoopBody
      (bind _asbp_props_gun_rifle (Utilities|Casting|CastToBP_Props_Gun_Rifle (.WeaponRef (Utilities|Struct|BreakStruct_WeaponState _array_element))))
      (Variables|/Game/BP/Props/Weapons/Gun/BP_Props_Gun.BP_Props_Gun_C|SetBulletNum _asbp_props_gun_rifle (+ (Variables|/Game/BP/Props/Weapons/Gun/BP_Props_Gun.BP_Props_Gun_C|GetBulletNum _asbp_props_gun_rifle) (Variables|Default|GetAddBulletNum)))
      (Actor|DestroyActor)
      (goto _label Break))))

(event EventRenderBegin
  (Rendering|SetRenderCustomDepth (Variables|Default|GetRamp_StaticMesh) true))

(event EventRenderEnd
  (Rendering|SetRenderCustomDepth (Variables|Default|GetRamp_StaticMesh) false))

(fn ConstructionScript
  (|CallParentFunction))