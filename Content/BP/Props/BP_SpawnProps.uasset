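; Spawner Blueprint whose events place medical items, weapons, ammo pickups, small AI enemies and a boss at given locations.
; Props scatter randomly in a flat box around the location, with ammo amounts passed into each bullet pickup.
; Enemies spawn at random navigable points within a radius, retrying without limit until a collision-checked spawn succeeds.
; Small-AI loops start at zero, apparently spawning one more of each type than requested if bounds are inclusive.
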(event Custom|SpawnMedical
  (params (MedicalAid :type Integer) (FirstAid :type Integer) (Serum :type Integer) (Bandgage :type Integer) (Location :type Vector))
  ;[1 1 1] Medical
  (Variables|Default|SetMedicalLocation Location)
  (Utilities|FlowControl|Sequence
    (:then_0
      (for _index (range 1 MedicalAid)
        (Utilities|SpawnWay "/Game/BP/Props/Medical/BP_Props_Medical_MedicalAid.BP_Props_Medical_MedicalAid_C" (Variables|Default|GetMedicalLocation))))
    (:then_1
      (for _index_2 (range 1 FirstAid)
        (Utilities|SpawnWay "/Game/BP/Props/Medical/BP_Props_Medical_FirstAid.BP_Props_Medical_FirstAid_C" (Variables|Default|GetMedicalLocation))))
    (:then_2
      (for _index_3 (range 1 Serum)
        (Utilities|SpawnWay "/Game/BP/Props/Medical/BP_Props_Medical_Serum.BP_Props_Medical_Serum_C" (Variables|Default|GetMedicalLocation))))
    (:then_3
      (for _index_4 (range 1 Bandgage)
        (Utilities|SpawnWay "/Game/BP/Props/Medical/BP_Props_Medical_Bandage.BP_Props_Medical_Bandage_C" (Variables|Default|GetMedicalLocation))))))

(event Custom|SpawnWeapon
  (params (Rifle :type Boolean) (Pistol :type Boolean) (Sword :type Boolean) (Location :type Vector))
  ;[1 1 1] Weapon
  (Variables|Default|SetWeaponLocation Location)
  (Utilities|FlowControl|Sequence
    (:then_0
      (if Rifle
        (Utilities|SpawnWay "/Game/BP/Props/Weapons/Gun/BP_Props_Gun_Rifle.BP_Props_Gun_Rifle_C" (Variables|Default|GetWeaponLocation))))
    (:then_1
      (if Pistol
        (Utilities|SpawnWay "/Game/BP/Props/Weapons/Gun/BP_Props_Gun_Pistol.BP_Props_Gun_Pistol_C" (Variables|Default|GetWeaponLocation))))
    (:then_2
      (if Sword
        (Utilities|SpawnWay "/Game/BP/Props/Weapons/Sword/BP_Props_Sword_Knife.BP_Props_Sword_Knife_C" (Variables|Default|GetWeaponLocation))))))

(event Custom|SpawnBullet
  (params (Rifle :type Integer) (Pistol :type Integer) (BulletLocation :type Vector))
  (bind _returnvalue (Math|Random|RandomPointinBoundingBox BulletLocation "100.000000,100.000000, 0"))
  (bind _returnvalue_2 (Math|Transform|MakeTransform _returnvalue))
  ;[1 1 1] Bullet
  (Utilities|FlowControl|Sequence
    (:then_0
      (if (!= Rifle 0)
        (Game|SpawnActorfromClass "/Game/BP/Props/BulleuBox/BP_Props_RifleBullet.BP_Props_RifleBullet_C" _returnvalue_2 "Undefined" 0 Rifle 0)))
    (:then_1
      (if (!= Pistol 0)
        (Game|SpawnActorfromClass "/Game/BP/Props/BulleuBox/BP_Props_PistolBullet.BP_Props_PistolBullet_C" _returnvalue_2 "Undefined" 0 Pistol 0)))))

(event Custom|SpawnAIBoss
  (params (Origin :type Vector%20%28by%20ref%29) (Radius :type Float%20%28single-precision%29))
  (bind _returnvalue (Game|SpawnActorfromClass "/Game/AI/Werewolf/BP_Boss.BP_Boss_C" (Math|Transform|MakeTransform (.RandomLocation (Class|NavigationSystemV1|GetRandomPointinNavigableRadius Origin Radius 0 0))) "AdjustIfPossibleButDontSpawnIfColliding" 0 0 :!label _label))
  (Utilities|IsValid _returnvalue
    (:Is%20Not%20Valid
      (goto _label))))

(event Custom|SpawnAISmall
  (params (Origin :type Vector%20%28by%20ref%29) (Radius :type Float%20%28single-precision%29) (Burst :type Integer) (GunZombie :type Integer) (Zombie :type Integer))
  (Variables|Default|SetAISmallLocation Origin)
  (Variables|Default|SetAiSmallRedius Radius)
  (Utilities|FlowControl|Sequence
    (:then_0
      (for _index (range 0 Burst)
        (bind _returnvalue (Utilities|SpawnAi "/Game/AI/Burst/BP_Burst.BP_Burst_C" :!label _label))
        (if (not _returnvalue)
          (goto _label))))
    (:then_1
      (for _index_2 (range 0 GunZombie)
        (bind _returnvalue_2 (Utilities|SpawnAi "/Game/AI/GunZombie/BP_GunZombie.BP_GunZombie_C" :!label _label_2))
        (if (not _returnvalue_2)
          (goto _label_2))))
    (:then_2
      (for _index_3 (range 0 Zombie)
        (bind _returnvalue_3 (Utilities|SpawnAi "/Game/AI/Zombie/BP_Zombie.BP_Zombie_C" :!label _label_3))
        (if (not _returnvalue_3)
          (goto _label_3))))))

(fn ConstructionScript)