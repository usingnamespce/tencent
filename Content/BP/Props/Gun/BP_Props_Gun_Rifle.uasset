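; BP_Props_Gun_Rifle is a rifle prop whose Fire event plays a shot sound and spawns a BP_Bullet_Test projectile from its BulletLocation.
; A Visibility trace from the player's follow camera finds the aim point, and the bullet is rotated from the muzzle toward the hit, correcting camera-to-muzzle offset.
; When the trace misses, the bullet uses the player's control rotation.
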(event EventFire
  (bind _player (Variables|Default|GetPlayer))
  (bind _bulletlocation (Variables|Default|GetBulletLocation))
  (bind _returnvalue (Transformation|GetWorldLocation _bulletlocation))
  (bind _followcamera (Variables|/Script/AndroidTest.AndroidTestCharacter|GetFollowCamera _player))
  (bind _returnvalue_2 (Transformation|GetWorldLocation _followcamera))
  (Audio|PlaySoundatLocation "/Game/Audio/Audio_Fire.FirstPersonTemplateWeaponFire02" _returnvalue_2 "0, 0, 0" 1.0 1.0 0.0 0 0 0)
  (bind (_outhit _returnvalue_3) (Collision|LineTraceByChannel _returnvalue_2 (+ _returnvalue_2 (* (Math|Vector|GetForwardVector (Transformation|GetWorldRotation _followcamera)) 6e+03)) "TraceTypeQuery1" false (Utilities|Array|MakeArray self) "None"))
  (if _returnvalue_3
    (Variables|Default|SetBulletRotation (Math|Rotator|FindLookatRotation _returnvalue (.Location (Collision|BreakHitResult _outhit))))
    (else
      (Variables|Default|SetBulletRotation (Pawn|GetControlRotation (Variables|Default|GetPlayer) :!class /Script/Engine.Pawn))))
  (Game|SpawnActorfromClass "/Game/Character/BP/BP_Bullet_TEst.BP_Bullet_Test_C" (Math|Transform|MakeTransform _returnvalue (Variables|Default|GetBulletRotation)) "Undefined" 0 0))

(fn ConstructionScript
  (|CallParentFunction))