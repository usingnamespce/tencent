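; BP_Props_Gun is a gun prop that the player can pick up as a weapon.
; RenderBegin and RenderEnd toggle custom depth on its static mesh, the usual hook for an outline highlight.
; PickUp passes the weapon name, socket name and a self reference to the player's AddGun.
; Fire is an empty event, while BeginPlay and construction only call the parent class.
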(event Custom|Fire)

(event EventBeginPlay
  (|CallParentFunction))

(event EventPickUp
  (Default|AddGun (Variables|Default|GetPlayer) (Variables|Default|GetName) (Variables|Default|GetSocketName) self))

(event EventRenderBegin
  (Rendering|SetRenderCustomDepth (Variables|Default|GetStaticMesh) true))

(event EventRenderEnd
  (Rendering|SetRenderCustomDepth (Variables|Default|GetStaticMesh) false))

(fn ConstructionScript
  (|CallParentFunction))