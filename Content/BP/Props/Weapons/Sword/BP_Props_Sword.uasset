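; Sword weapon prop Blueprint that controls the highlighting and visibility of its static and skeletal meshes.
; RenderBegin and RenderEnd toggle custom depth rendering on the static mesh.
; HiddenSelf swaps representations by showing the skeletal mesh and hiding the static mesh, without propagating to children.
; BeginPlay and the construction script only defer to the parent class.
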(event EventBeginPlay
  (|CallParentFunction))

(event EventRenderBegin
  (Rendering|SetRenderCustomDepth (Variables|Default|GetStaticMesh) true))

(event EventRenderEnd
  (Rendering|SetRenderCustomDepth (Variables|Default|GetStaticMesh) false))

(event EventHiddenSelf
  (Rendering|SetVisibility (Variables|Default|GetSkeletalMesh) true false)
  (Rendering|SetVisibility (Variables|Default|GetStaticMesh) false false))

(fn ConstructionScript
  (|CallParentFunction))