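; Knife weapon prop with a melee attack that damages pawns.
; Attack calls AttackServer, which plays the attack montage and calls AttackClient to replay it on non-authority machines.
; Between the montage's notify begin and end, a looping timer line-traces from previous to current points interpolated between two blade sockets, catching hits along the swept path.
; A DoOnce, reset at each notify begin, limits damage to one hit per window.
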(event Custom|AttackServer
  (params (Player :type BP%20Character%20Object%20Reference))
  (Animation|Montage|PlayMontage (Variables|/Script/Engine.Character|GetMesh Player) "/Game/Character/Animations/Montage/Twinblades_attack02_Montage.Twinblades_attack02_Montage"
    (:then
      (CallFunction|AttackClient Player))
    (:OnNotifyBegin
      (bind _locations (CallFunction|GetLocationforKnife 5))
      (Variables|Default|SetLastLocations _locations)
      (bind _returnvalue (Utilities|Time|SetTimerbyEvent (delegate Custom|BeginTrack) 0.01 true))
      (Variables|Default|SetAttackHandle _returnvalue)
      (Utilities|FlowControl|DoOnce false) ; enters at Reset
    )
    (:OnNotifyEnd
      (Utilities|Time|ClearandInvalidateTimerbyHandle (Variables|Default|GetAttackHandle)))))

(event Custom|AttackClient
  (params (Player :type BP%20Character%20Object%20Reference))
  (Networking|SwitchHasAuthority
    (:Remote
      (Animation|Montage|PlayMontage (Variables|/Script/Engine.Character|GetMesh Player) "/Game/Character/Animations/Montage/Twinblades_attack02_Montage.Twinblades_attack02_Montage"))))

(event Custom|BeginTrack
  (bind _locations (CallFunction|GetLocationforKnife 5))
  (bind _output_get (Variables|Default|SetNowLocations _locations))
  (for (_array_element _array_index) _output_get
    (bind (_outhit _returnvalue) (Collision|LineTraceForObjects (Utilities|Array|Get(acopy) (Variables|Default|GetLastLocations) _array_index) _array_element (Utilities|Array|MakeArray "ObjectTypeQuery3") false 0 "None"))
    (if _returnvalue
      (Utilities|FlowControl|DoOnce false
        (:Completed
          (Game|Damage|ApplyDamage (.HitActor (Collision|BreakHitResult _outhit)) 5e+01 (Pawn|GetController (.AsBP%20Character (Utilities|Casting|CastToBP_Character (Components|GetOwner)))) 0)))))
  (Variables|Default|SetLastLocations (Variables|Default|GetNowLocations)))

(event EventBeginPlay
  (|CallParentFunction) ; 此节点被禁用，将不会被调用。\n从引脚连出引线来编译功能。
)

(event EventAttack
  (CallFunction|AttackServer (Variables|Default|GetPlayer)))

(fn ConstructionScript
  (|CallParentFunction))

(fn GetLocationforKnife
  (params (Parts :type Integer))
  (bind _skeletalmesh (Variables|Default|GetSkeletalMesh))
  (bind _output_get (LocalVariables|SetPartNum (- Parts 1)))
  (for _index (range 1 _output_get)
    (Utilities|Array|Add (LocalVariables|GetLocation) (+ (* (.Location (Math|Transform|BreakTransform (Transformation|GetSocketTransform _skeletalmesh "SocketTwo" "RTS_World"))) (/ (Math|Conversions|ToFloat(Integer) _index) (Math|Conversions|ToFloat(Integer) (LocalVariables|GetPartNum)))) (* (.Location (Math|Transform|BreakTransform (Transformation|GetSocketTransform _skeletalmesh "SocketOne" "RTS_World"))) (- 1.0 (/ (Math|Conversions|ToFloat(Integer) _index) (Math|Conversions|ToFloat(Integer) (LocalVariables|GetPartNum))))))))
  (return (LocalVariables|GetLocation)))