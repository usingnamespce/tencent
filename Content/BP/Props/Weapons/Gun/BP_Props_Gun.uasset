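; Gun weapon prop Blueprint that handles the gun's mesh display and highlight state.
; RenderBegin and RenderEnd toggle custom depth rendering on the static mesh.
; HiddenSelf swaps visibility from the static mesh to the skeletal mesh, without propagating to children.
; Reload is an empty stub, while BeginPlay and construction only call the parent.
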(event Custom|Reload)

(event EventBeginPlay
  (|CallParentFunction))

(event EventHiddenSelf
  (Rendering|SetVisibility (Variables|Default|GetSkeletalMesh) true false)
  (Rendering|SetVisibility (Variables|Default|GetStaticMesh) false false))

(event EventRenderBegin
  (Rendering|SetRenderCustomDepth (Variables|Default|GetStaticMesh) true))

(event EventRenderEnd
  (Rendering|SetRenderCustomDepth (Variables|Default|GetStaticMesh) false))

(fn ConstructionScript
  (|CallParentFunction))