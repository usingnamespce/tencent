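; Rifle weapon prop that fires projectile bullets and manages magazine and reserve ammo.
; Attack checks fire interval and magazine count, then traces from the player's camera to aim the muzzle at the hit point, falling back to control rotation.
; Server-to-client event pairs relay the shot sound, bullet spawn and reload montage.
; When the montage completes, only the locally controlled player refills the magazine from reserve.
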(event Custom|FireClient
  (params (Transform :type Transform) (Location :type Vector))
  (bind _returnvalue (Components|GetOwner))
  ;[1 1 1] Fire
  (Audio|PlaySoundatLocation "/Game/Audio/Audio_Fire.FirstPersonTemplateWeaponFire02" Location "0, 0, 0" 1.0 1.0 0.0 0 0 0)
  (Game|SpawnActorfromClass "/Game/Character/BP/BP_Bullet_TEst.BP_Bullet_Test_C" Transform "Undefined" _returnvalue (.AsBP%20Character (Utilities|Casting|CastToBP_Character _returnvalue))))

(event Custom|FireServer
  (params (Transform :type Transform) (Location :type Vector))
  ;[1 1 1] Fire
  (CallFunction|FireClient Transform Location))

(event Custom|Fire
  (bind _player (Variables|Default|GetPlayer))
  (bind _bulletlocation (Variables|Default|GetBulletLocation))
  (bind _returnvalue (Transformation|GetWorldLocation _bulletlocation))
  (bind _camera (Variables|/Game/Character/BP/BP_Character.BP_Character_C|GetCamera _player))
  (bind _returnvalue_2 (Transformation|GetWorldLocation _camera))
  ;[1 1 1] Fire
  (bind _output_get (Variables|Default|SetLocation _returnvalue_2))
  (bind (_outhit _returnvalue_3) (Collision|LineTraceByChannel _output_get (+ _returnvalue_2 (* (Math|Vector|GetForwardVector (Transformation|GetWorldRotation _camera)) 6e+03)) "TraceTypeQuery1" false (Utilities|Array|MakeArray self) "None"))
  (if _returnvalue_3
    (Variables|Default|SetBulletRotation (Math|Rotator|FindLookatRotation _returnvalue (.Location (Collision|BreakHitResult _outhit))))
    (else
      (Variables|Default|SetBulletRotation (Pawn|GetControlRotation (Variables|Default|GetPlayer) :!class /Script/Engine.Pawn))))
  (CallFunction|FireServer (Math|Transform|MakeTransform _returnvalue (Variables|Default|GetBulletRotation)) (Variables|Default|GetLocation)))

(event Custom|ReloadMontageClient
  (params (目标 :type Character%20Object%20Reference))
  ;[1 1 1] Reload
  (Animation|Montage|PlayMontage (Variables|/Script/Engine.Character|GetMesh 目标) "/Game/Character/Animations/Montage/Reload_Pistol_Montage.Reload_Pistol_Montage"
    (:OnCompleted
      (if (Pawn|IsLocallyControlled 目标)
        (CallFunction|ReloadBulletHandle)))))

(event Custom|ReloadMontageServer
  (params (目标 :type Character%20Object%20Reference))
  ;[1 1 1] Reload
  (CallFunction|ReloadMontageClient 目标))

(event EventAttack
  ;[1 1 1] Fire
  (if (CallFunction|CanFire)
    (CallFunction|Fire)
    (Math|Integer|DecrementInt (Variables|Default|GetBulletCartridgeNum))))

(event EventReload
  ;[1 1 1] Reload
  (if (and (> (Variables|Default|GetBulletNum) 0) (< (Variables|Default|GetBulletCartridgeNum) 30))
    (CallFunction|ReloadMontageServer (Variables|Default|GetPlayer))))

(fn ConstructionScript
  (|CallParentFunction))

(fn CanFire
  (bind _output_get (LocalVariables|SetCanFireByTime (>= (- (Utilities|Time|GetGameTimeinSeconds) (Variables|Default|GetLastFireTime)) (Variables|Default|GetFireTime))))
  (if _output_get
    (Variables|Default|SetLastFireTime (Utilities|Time|GetGameTimeinSeconds)))
  (return (and (> (Variables|Default|GetBulletCartridgeNum) 0) (LocalVariables|GetCanFireByTime))))

(fn ReloadBulletHandle
  (if (<= (- (Variables|Default|GetMaxBulletCartridgeNum) (Variables|Default|GetBulletCartridgeNum)) (Variables|Default|GetBulletNum))
    (Variables|Default|SetBulletNum (- (Variables|Default|GetBulletNum) (- (Variables|Default|GetMaxBulletCartridgeNum) (Variables|Default|GetBulletCartridgeNum))))
    (Variables|Default|SetBulletCartridgeNum (Variables|Default|GetMaxBulletCartridgeNum))
    (else
      (Variables|Default|SetBulletCartridgeNum (+ (Variables|Default|GetBulletCartridgeNum) (Variables|Default|GetBulletNum)))
      (Variables|Default|SetBulletNum 0))))