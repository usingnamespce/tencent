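; BP_Zombie is a zombie AI character with a montage-driven melee attack against BP_Character targets.
; Attack calls AttackClient, which plays a randomly chosen attack section and uses its notify window to toggle Left and Right hit collision.
; A fast looping timer runs during that window, while AttackJudge gathers unique overlapping targets per side.
; When the window ends, collected targets take damage and the target lists are cleared.
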(event Custom|AttackClient
  (bind _damage (Variables|Default|GetDamage))
  (Animation|Montage|PlayMontage (Variables|Character|GetMesh) "/Game/AI/Zombie/Animations/Attack_Zombie.Attack_Zombie" 1.0 0.0 (Utilities|String|StringToName (Utilities|String|Append (Utilities|String|ToString(Name) (Utilities|Name|MakeLiteralName "Attack")) (Utilities|String|ToString(Integer) (Math|Random|RandomIntegerinRange 1 3))))
    (:OnNotifyBegin
      (Collision|SetCollisionEnabled (Variables|Default|GetLeft) "QueryOnly")
      (bind _returnvalue (Utilities|Time|SetTimerbyEvent (EventDispatchers|CreateEvent :!event Custom|AttackJudge) 0.01 true))
      (Variables|Default|SetAttackHandle _returnvalue))
    (:OnNotifyEnd
      (Collision|SetCollisionEnabled (Variables|Default|GetLeft) "NoCollision")
      (Utilities|Time|ClearandInvalidateTimerbyHandle (Variables|Default|GetAttackHandle))
      (Utilities|FlowControl|Sequence
        (:then_0
          (for _array_element (Variables|Default|GetAttackTargetLeft)
            (Game|Damage|ApplyDamage _array_element _damage 0 0))
          (Utilities|Array|Clear (Variables|Default|GetAttackTargetLeft)))
        (:then_1
          (for _array_element_2 (Variables|Default|GetAttackTargetRight)
            (Game|Damage|ApplyDamage _array_element_2 _damage 0 0)
            (Utilities|Array|Clear (Variables|Default|GetAttackTargetRight))))))))

(event Custom|AttackJudge
  (for _array_element (Collision|GetOverlappingActors (Variables|Default|GetRight) "/Game/Character/BP/BP_Character.BP_Character_C" :!class /Script/Engine.PrimitiveComponent)
    (Utilities|Array|AddUnique (Variables|Default|GetAttackTargetRight) _array_element))
  (for _array_element_2 (Collision|GetOverlappingActors (Variables|Default|GetLeft) "/Game/Character/BP/BP_Character.BP_Character_C" :!class /Script/Engine.PrimitiveComponent)
    (Utilities|Array|AddUnique (Variables|Default|GetAttackTargetLeft) _array_element_2)))

(event EventAttack
  (CallFunction|AttackClient))

(fn ConstructionScript
  (|CallParentFunction))