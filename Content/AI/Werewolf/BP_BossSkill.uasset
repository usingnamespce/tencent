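; BP_BossSkill is a damage-area actor for a boss skill, filed under the Werewolf AI.
; On BeginPlay, only the authority starts a looping timer at the DamageTime interval.
; Each tick of that timer applies BaseDamage to every BP_Character overlapping its Box.
; In parallel, a delay of LifeTime destroys the actor, without an authority check.
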(event Custom|自定义事件_0
  (for _array_element (Collision|GetOverlappingActors (Variables|Default|GetBox) "/Game/Character/BP/BP_Character.BP_Character_C" :!class /Script/Engine.PrimitiveComponent)
    (Game|Damage|ApplyDamage _array_element (Variables|Default|GetBase%20Damage) 0 0)))

(event EventBeginPlay
  (Utilities|FlowControl|Sequence
    (:then_0
      (Networking|SwitchHasAuthority
        (:Authority
          (Utilities|Time|SetTimerbyEvent (delegate Custom|自定义事件_0) (Variables|Default|GetDamageTime) true))))
    (:then_1
      (Utilities|FlowControl|Delay (Variables|Default|GetLifeTime))
      (Actor|DestroyActor))))

(fn ConstructionScript)