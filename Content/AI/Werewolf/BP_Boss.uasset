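; Werewolf boss character driven by a server-run behavior tree, with a life widget, start and death sounds.
; Jump and melee montage notifies open hand-collision windows and damage collected targets on close; ranged attacks spawn bullets.
; Damage retargets the instigator, and low life triggers a one-time howl spawning skill actors at the target and random navmesh points.
; Death awards score, drops medical items, weapons and ammo, then destroys the boss after a delay.
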(event Custom|AttackJudge
  (bind _attacktargetright (Variables|Default|GetAttackTargetRight))
  (bind _left (Variables|Default|GetLeft))
  (bind _right (Variables|Default|GetRight))
  (bind _attacktargetleft (Variables|Default|GetAttackTargetLeft))
  ;[1 1 1] Normal Attack
  ;;[0 0 0] Damage judge
  (for _array_element (Collision|GetOverlappingActors _right "/Game/Character/BP/BP_Character.BP_Character_C" :!class /Script/Engine.PrimitiveComponent)
    (Utilities|Array|AddUnique _attacktargetright _array_element))
  (Utilities|Array|AppendArray _attacktargetright (Collision|GetOverlappingActors _right "/Game/AI/NPC/BP_NPC.BP_NPC_C" :!class /Script/Engine.PrimitiveComponent))
  (for _array_element_2 (Collision|GetOverlappingActors _left "/Game/Character/BP/BP_Character.BP_Character_C" :!class /Script/Engine.PrimitiveComponent)
    (Utilities|Array|AddUnique _attacktargetleft _array_element_2))
  (Utilities|Array|AppendArray _attacktargetleft (Collision|GetOverlappingActors _left "/Game/AI/NPC/BP_NPC.BP_NPC_C" :!class /Script/Engine.PrimitiveComponent)))

(event Custom|onDamageClient
  (params (Instigated%20By :type Controller%20Object%20Reference) (B :type Float%20%28single-precision%29))
  (bind _returnvalue (AI|GetBlackboard 0))
  (bind _lifewidger (Variables|Default|GetLifeWidger))
  (bind _mesh (Variables|Character|GetMesh))
  (bind _returnvalue_2 (Transformation|GetWorldLocation _mesh))
  ;[1 1 1] onHit
  (Variables|Default|SetInstigated%20By Instigated%20By)
  (Variables|Default|SetLife (- (Variables|Default|GetLife) B))
  (if (<= (Variables|Default|GetLife) 0.0)
    (Variables|Default|SetisDeath true)
    (CallFunction|DeathHandle (Variables|Default|GetInstigated%20By))
    (Utilities|FlowControl|Sequence
      (:then_0
        (Utilities|IsValid _returnvalue
          (:Is%20Valid
            (AI|Components|Blackboard|SetValueasBool _returnvalue (Utilities|Name|MakeLiteralName "isDeath") true))))
      (:then_1
        (Utilities|IsValid _lifewidger
          (:Is%20Valid
            (Widget|RemovefromParent _lifewidger)
            (Networking|SwitchHasAuthority
              (:Authority
                (bind _outactors (Actor|GetAllActorsOfClass "/Game/BP/Props/BP_SpawnProps.BP_SpawnProps_C"))
                (Default|SpawnMedical (Utilities|Array|Get(acopy) _outactors) 1 1 1 1 _returnvalue_2)
                (Default|SpawnWeapon (Utilities|Array|Get(acopy) _outactors) true true true _returnvalue_2)
                (Default|SpawnBullet (Utilities|Array|Get(acopy) _outactors) 100 50 _returnvalue_2)
                (Utilities|FlowControl|Delay 1e+01)
                (Actor|DestroyActor))))))
      (:then_2
        (Audio|PlaySoundatLocation "/Game/Audio/Boss/Boss_Death.Boss_Death" (Transformation|GetActorLocation) "0, 0, 0" 1.0 1.0 0.0 0 0 0)))
    (else
      ;[1 1 1] Skill
      (Networking|SwitchHasAuthority
        (:Authority
          (if (<= (Variables|Default|GetLife) 5e+01)
            (Utilities|FlowControl|DoOnce false
              (:Completed
                (Utilities|Array|Add (Variables|Skill|GetSpawn%20Transform) (Math|Transform|MakeTransform (Transformation|GetActorLocation (.AsActor (Utilities|Casting|CastToActor (AI|Components|Blackboard|GetValueasObject (AI|GetBlackboard 0) (Utilities|Name|MakeLiteralName "AttackTarget"))))) "0, 0, 0" "0.500000,0.500000,0.500000"))
                (for _index (range 0 (- (Variables|Skill|GetNum) 2))
                  (bind _randomlocation (Class|NavigationSystemV1|GetRandomLocationinNavigableRadius (Transformation|GetActorLocation) (Variables|Skill|GetRadius) 0 0))
                  (Utilities|Array|Add (Variables|Skill|GetSpawn%20Transform) (Math|Transform|MakeTransform _randomlocation "0, 0, 0" "0.500000,0.500000,0.500000")))
                (CallFunction|Skill (Variables|Skill|GetSpawn%20Transform))))))))))

(event Custom|Skill
  (params (SpawnTransform :type Array%20of%20Transforms))
  ;[1 1 1] Skill
  (Animation|Montage|PlayMontage (Variables|Character|GetMesh) "/Game/AI/Werewolf/Animations/ANIM_WEREWOLF_howl_Montage.ANIM_WEREWOLF_howl_Montage"
    (:then
      (Audio|PlaySoundatLocation "/Game/Audio/Boss/Boss_Skills.Boss_Skills" (Transformation|GetActorLocation) "0, 0, 0" 1.0 1.0 0.0 0 0 0))
    (:OnBlendOut
      (for _array_element SpawnTransform :!label _label
        (Game|SpawnActorfromClass "/Game/AI/Werewolf/BP_BossSkill.BP_BossSkill_C" _array_element "Undefined" 0 0)))
    (:OnInterrupted
      (goto _label))))

(event Custom|AttackClient
  (params (isRomote :type Boolean) (SpawnTransform :type Transform) (StartingSection :type Name))
  (bind _damage (Variables|Default|GetDamage))
  ;[1 1 1] Normal Attack
  (if isRomote
    (Animation|Montage|PlayMontage (Variables|Character|GetMesh) "/Game/AI/Werewolf/Animations/AttackRomote_Boss.AttackRomote_Boss" 1.0 0.0 StartingSection
      (:OnBlendOut
        (Game|SpawnActorfromClass "/Game/AI/Werewolf/BP_BossBullet.BP_BossBullet_C" SpawnTransform "Undefined" 0 (Variables|Default|GetDamage) 0)))
    (else
      (Animation|Montage|PlayMontage (Variables|Character|GetMesh) "/Game/AI/Werewolf/Animations/AttackFWd_Boss.AttackFWd_Boss" 1.0 0.0 StartingSection
        (:OnInterrupted
          (Utilities|Time|ClearandInvalidateTimerbyHandle (Variables|Default|GetAttackHandle)))
        (:OnNotifyBegin
          (Collision|SetCollisionEnabled (Variables|Default|GetLeft) "QueryOnly")
          (bind _returnvalue (Utilities|Time|SetTimerbyEvent (EventDispatchers|CreateEvent :!event Custom|AttackJudge) 0.01 true))
          (Variables|Default|SetAttackHandle _returnvalue))
        (:OnNotifyEnd
          (Collision|SetCollisionEnabled (Variables|Default|GetLeft) "NoCollision")
          (Utilities|Time|ClearandInvalidateTimerbyHandle (Variables|Default|GetAttackHandle))
          (Utilities|FlowControl|Sequence
            (:then_0
              (for _array_element (Variables|Default|GetAttackTargetLeft)
                (Game|Damage|ApplyDamage _array_element _damage 0 0))
              (Utilities|Array|Clear (Variables|Default|GetAttackTargetLeft)))
            (:then_1
              (for _array_element_2 (Variables|Default|GetAttackTargetRight)
                (Game|Damage|ApplyDamage _array_element_2 _damage 0 0))
              (Utilities|Array|Clear (Variables|Default|GetAttackTargetRight)))))))))

(event Custom|Attack
  (params (isRomote :type Boolean))
  (bind _returnvalue (Utilities|Name|MakeLiteralName "AttackTarget"))
  (bind _self self)
  (bind _returnvalue_2 (AI|GetBlackboard _self))
  (bind _returnvalue_3 (AI|Components|Blackboard|GetValueasObject _returnvalue_2 _returnvalue))
  (bind _asactor (Utilities|Casting|CastToActor _returnvalue_3))
  (bind _returnvalue_4 (Transformation|GetActorLocation _asactor))
  ;[1 1 1] Normal Attack
  (CallFunction|AttackClient isRomote (Math|Transform|MakeTransform (Transformation|GetWorldLocation (Variables|Default|GetArrow1)) (Math|Rotator|FindLookatRotation (Transformation|GetWorldLocation (Variables|Default|GetArrow1)) (Math|Vector|MakeVector (.x _returnvalue_4) (.y _returnvalue_4) (+ (.z _returnvalue_4) 3e+01))) "0.500000,0.500000,0.500000") (Utilities|String|StringToName (Utilities|String|Append (Utilities|String|ToString(Name) (Utilities|Name|MakeLiteralName "Attack")) (Utilities|String|ToString(Integer) (Math|Random|RandomIntegerinRange 1 3))))))

(event Custom|JumpAttackClient
  (bind _damage (Variables|Default|GetDamage))
  ;[1 1 1] Jump Attack
  (Animation|Montage|PlayMontage (Variables|Character|GetMesh) "/Game/AI/Werewolf/Animations/AttackJump_Boss.AttackJump_Boss" 1.0 0.0 (Utilities|String|StringToName (Utilities|String|Append (Utilities|String|ToString(Name) (Utilities|Name|MakeLiteralName "Attack")) (Utilities|String|ToString(Integer) (Math|Random|RandomIntegerinRange 1 2))))
    (:OnInterrupted
      (Utilities|Time|ClearandInvalidateTimerbyHandle (Variables|Default|GetAttackHandle)))
    (:OnNotifyBegin
      (Collision|SetCollisionEnabled (Variables|Default|GetLeft) "QueryOnly")
      (bind _returnvalue (Utilities|Time|SetTimerbyEvent (EventDispatchers|CreateEvent :!event Custom|AttackJudge) 0.01 true))
      (Variables|Default|SetAttackHandle _returnvalue))
    (:OnNotifyEnd
      (Collision|SetCollisionEnabled (Variables|Default|GetLeft) "NoCollision")
      (Utilities|Time|ClearandInvalidateTimerbyHandle (Variables|Default|GetAttackHandle))
      (Utilities|FlowControl|Sequence
        (:then_0
          (for _array_element (Variables|Default|GetAttackTargetLeft)
            (Game|Damage|ApplyDamage _array_element _damage 0 0))
          (Utilities|Array|Clear (Variables|Default|GetAttackTargetLeft)))
        (:then_1
          (for _array_element_2 (Variables|Default|GetAttackTargetRight)
            (Game|Damage|ApplyDamage _array_element_2 _damage 0 0)
            (Utilities|Array|Clear (Variables|Default|GetAttackTargetRight))))))))

(event Custom|JumpAttack
  ;[1 1 1] Jump Attack
  (CallFunction|JumpAttackClient))

(event Game|Damage|EventAnyDamage
  (params (Damage :type Float%20%28single-precision%29) (DamageType :type Damage%20Type%20Object%20Reference) (InstigatedBy :type Controller%20Object%20Reference) (DamageCauser :type Actor%20Object%20Reference))
  (bind _returnvalue (AI|GetBlackboard 0))
  ;[1 1 1] onHit
  (if (not (Variables|Default|GetisDeath))
    (CallFunction|OnDamageClient InstigatedBy Damage)
    (Utilities|IsValid _returnvalue
      (:Is%20Valid
        (AI|Components|Blackboard|SetValueasObject _returnvalue (Utilities|Name|MakeLiteralName "AttackTarget") (Pawn|GetControlledPawn InstigatedBy))))))

(event EventBeginPlay
  (bind _self self)
  (bind _returnvalue (AI|GetAIController _self))
  ;[1 1 1] Begin
  (Utilities|FlowControl|Sequence
    (:then_0
      (Networking|SwitchHasAuthority
        (:Authority
          (AI|RunBehaviorTree _returnvalue "/Game/AI/Werewolf/Control/BT_Boss.BT_Boss")
          (Class|AIController|UseBlackboard _returnvalue "/Game/AI/Werewolf/Control/BB_Boss.BB_Boss"))))
    (:then_1
      (bind _returnvalue_2 (UserInterface|CreateWidget "/Game/BP/Widget/UMG_BossLife.UMG_BossLife_C" 0 self))
      (bind _output_get (Variables|Default|SetLifeWidger _returnvalue_2))
      (UserInterface|Viewport|AddtoViewport _output_get 0)
      (Audio|PlaySoundatLocation "/Game/Audio/Boss/Boss_Start.Boss_Start" (Transformation|GetActorLocation) "0, 0, 0" 1.0 1.0 0.0 0 0 0))))

(fn ConstructionScript)

(fn DeathHandle
  (params (Instigated%20By :type Controller%20Object%20Reference))
  (bind _asbp_my_player_control (Utilities|Casting|CastToBP_MyPlayerControl Instigated%20By))
  (bind _asbp_my_player_state (Utilities|Casting|CastToBP_MyPlayerState (Variables|/Script/Engine.Controller|GetPlayerState _asbp_my_player_control)))
  (Default|UpdateScore _asbp_my_player_state (Variables|Default|GetAddScore))
  (Collision|SetCollisionEnabled (Variables|Collision|GetCapsuleComponent) "NoCollision"))