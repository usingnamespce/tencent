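; Base character for small AI enemies, with health, death, score reward and an empty Attack event.
; On the authority it runs BT_AiSmall and sets the blackboard's isRomote flag from the "Romote" actor tag; construction applies MaxSpeed to walk speed.
; Damage makes the instigator's pawn the AttackTarget and reduces Life through onDamageClient.
; At zero Life it flags death in the blackboard and adds score to the instigating player's state.
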(event Custom|Attack)

(event Custom|onDamageClient
  (params (Instigated%20By :type Controller%20Object%20Reference) (Damage :type Float%20%28single-precision%29))
  (bind _returnvalue (AI|GetBlackboard 0))
  (Variables|Default|SetInstigated%20By Instigated%20By)
  (Variables|Default|SetLife (- (Variables|Default|GetLife) Damage))
  (if (<= (Variables|Default|GetLife) 0.0)
    (Variables|Default|SetisDeath true)
    (CallFunction|DeathHandle (Variables|Default|GetInstigated%20By))
    (Utilities|IsValid _returnvalue
      (:Is%20Valid
        (AI|Components|Blackboard|SetValueasBool _returnvalue (Utilities|Name|MakeLiteralName "isDeath") true)))))

(event Game|Damage|EventAnyDamage
  (params (Damage :type Float%20%28single-precision%29) (DamageType :type Damage%20Type%20Object%20Reference) (InstigatedBy :type Controller%20Object%20Reference) (DamageCauser :type Actor%20Object%20Reference))
  (if (not (Variables|Default|GetisDeath))
    (CallFunction|OnDamageClient InstigatedBy Damage)
    (AI|Components|Blackboard|SetValueasObject (AI|GetBlackboard 0) (Utilities|Name|MakeLiteralName "AttackTarget") (Pawn|GetControlledPawn InstigatedBy))))

(event EventBeginPlay
  (bind _self self)
  (bind _returnvalue (AI|GetAIController _self))
  (Networking|SwitchHasAuthority
    (:Authority
      (AI|RunBehaviorTree _returnvalue "/Game/AI/AiSmall/BT_AiSmall.BT_AiSmall")
      (bind _blackboardcomponent (Class|AIController|UseBlackboard _returnvalue "/Game/AI/AiSmall/BB_AiSmall.BB_AiSmall"))
      (AI|Components|Blackboard|SetValueasBool _blackboardcomponent (Utilities|Name|MakeLiteralName "isRomote") (Actor|ActorHasTag "Romote")))))

(fn ConstructionScript
  (Variables|/Script/Engine.CharacterMovementComponent|SetMaxWalkSpeed (Variables|Character|GetCharacterMovement) (Variables|Default|GetMaxSpeed)))

(fn DeathHandle
  (params (Instigated%20By :type Controller%20Object%20Reference))
  (bind _asbp_my_player_control (Utilities|Casting|CastToBP_MyPlayerControl Instigated%20By))
  (bind _asbp_my_player_state (Utilities|Casting|CastToBP_MyPlayerState (Variables|/Script/Engine.Controller|GetPlayerState _asbp_my_player_control)))
  (Default|UpdateScore _asbp_my_player_state (Variables|Default|GetAddScore)))