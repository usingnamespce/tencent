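; Gun-wielding zombie AI character that shoots bullets at its attack target.
; Attack reads the target actor from the Blackboard and builds a scaled spawn transform at an arrow component, aimed slightly above the target's location.
; AttackClient takes that transform, starts the attack montage, then immediately spawns a bullet carrying the zombie's damage and plays a firing sound at the spawn point.
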(event Custom|AttackClient
  (params (SpawnTransform :type Transform))
  (Animation|Montage|PlayMontage (Variables|Character|GetMesh) "/Game/AI/GunZombie/Animations/Attack_GunZombie.Attack_GunZombie"
    (:then
      (Game|SpawnActorfromClass "/Game/AI/GunZombie/BP_GunZombieBullet.BP_GunZombieBullet_C" SpawnTransform "Undefined" 0 (Variables|Default|GetDamage) 0)
      (Audio|SpawnSoundatLocation "/Game/Audio/Audio_Fire.FirstPersonTemplateWeaponFire02" (.Location (Math|Transform|BreakTransform SpawnTransform)) "0, 0, 0" 1.0 1.0 0.0 0 0))))

(event EventAttack
  (bind _returnvalue (Utilities|Name|MakeLiteralName "AttackTarget"))
  (bind _self self)
  (bind _returnvalue_2 (AI|GetBlackboard _self))
  (bind _returnvalue_3 (AI|Components|Blackboard|GetValueasObject _returnvalue_2 _returnvalue))
  (bind _asactor (Utilities|Casting|CastToActor _returnvalue_3))
  (bind _returnvalue_4 (Transformation|GetActorLocation _asactor))
  (CallFunction|AttackClient (Math|Transform|MakeTransform (Transformation|GetWorldLocation (Variables|Default|GetArrow1)) (Math|Rotator|FindLookatRotation (Transformation|GetWorldLocation (Variables|Default|GetArrow1)) (Math|Vector|MakeVector (.x _returnvalue_4) (.y _returnvalue_4) (+ (.z _returnvalue_4) 3e+01))) "5.000000,5.000000,5.000000")))

(fn ConstructionScript
  (|CallParentFunction))