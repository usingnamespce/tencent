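; BP_Burst is an AI self-destruct actor that explodes when Attack is called, damaging nearby BP_Character actors.
; Attack calls AttackClient, which uses a DoOnce and a timeline to swell the actor to 1.5x scale before spawning an explosion effect.
; It adds a sphere component at runtime, waits briefly, damages overlapping characters, then destroys itself.
; Only with authority, it also calls Blood on each victim's BP_MyPlayerState with duration and damage values.
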(event Custom|AttackClient
  (Utilities|FlowControl|DoOnce false
    (:Completed
      (bind _新建轨道_0 (Timeline|时间轴_0 PlayFromStart)
        (:Update
          (Transformation|SetActorScale3D (Math|Vector|Lerp(Vector) "1.000000,1.000000,1.000000" "1.500000,1.500000,1.500000" _新建轨道_0)))
        (:Finished
          (Effects|SpawnEmitteratLocation "/Game/FX/Burst/Particles/P_Explosion.P_Explosion" (Transformation|GetActorLocation) "0, 0, 0" "10.000000,10.000000,10.000000")
          (bind _returnvalue (AddComponent|AddSphereComponent false))
          (Utilities|FlowControl|Delay 0.5)
          (for _array_element (Collision|GetOverlappingActors _returnvalue "/Game/Character/BP/BP_Character.BP_Character_C" :!class /Script/Engine.PrimitiveComponent)
            (Game|Damage|ApplyDamage _array_element (Variables|Default|GetDamage) 0 0)
            (Networking|SwitchHasAuthority
              (:Authority
                (bind _asbp_character (Utilities|Casting|CastToBP_Character _array_element))
                (bind _asbp_my_player_state (Utilities|Casting|CastToBP_MyPlayerState (Variables|/Script/Engine.Pawn|GetPlayerState _asbp_character)))
                (Default|Blood _asbp_my_player_state (Variables|Default|GetBloodSecond) (Variables|Default|GetBloodDamage)))))
          (Actor|DestroyActor))))))

(event EventAttack
  (CallFunction|AttackClient))

(fn ConstructionScript
  (|CallParentFunction))