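; NPC spirit that wanders once started and loses the game for the player if it dies.
; StartMove plays a start sound, then on authority repeatedly moves to random reachable nearby points on a looping timer.
; Damage passes through DamageServerNPC to DamageClientNPC, which reduces Life and plays a rate-limited hit sound.
; When Life runs out, it calls EndGame on BP_MyGamemode with a failure result.
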(event Custom|Move
  (AI|AIMoveTo self (.RandomLocation (AI|Navigation|GetRandomReachablePointinRadius (Transformation|GetActorLocation) 3e+03 0 0)) 0 5.0 false))

(event Custom|DamageClientNPC
  (params (Damage :type Float%20%28single-precision%29))
  (bind _returnvalue (Utilities|Time|GetGameTimeinSeconds))
  (bind _output_get (Variables|Default|SetLife (- (Variables|Default|GetLife) Damage)))
  (if (<= _output_get 0.0)
    (bind _asbp_my_gamemode (Utilities|Casting|CastToBP_MyGamemode (Game|GetGameMode)))
    (Default|EndGame _asbp_my_gamemode "游戏失败，精灵死亡" false)
    (elif (> (- _returnvalue (Variables|Default|GetLastTime)) 2.0)
      (Variables|Default|SetLastTime _returnvalue)
      (Audio|PlaySoundatLocation "/Game/Audio/NPC/NPC_Hit.NPC_Hit" (Transformation|GetActorLocation) "0, 0, 0" 1.0 1.0 0.0 0 0 0))))

(event Custom|DamageServerNPC
  (params (Damage :type Float%20%28single-precision%29))
  (CallFunction|DamageClientNPC Damage))

(event Custom|StartMove
  (Audio|PlaySoundatLocation "/Game/Audio/NPC/NPC_StartGame.NPC_StartGame" (Transformation|GetActorLocation) "0, 0, 0" 1.0 1.0 0.0 0 0 0)
  (Networking|SwitchHasAuthority
    (:Authority
      (CallFunction|Move)
      (Utilities|Time|SetTimerbyEvent (delegate Custom|Move) 5.0 true))))

(event Game|Damage|EventAnyDamage
  (params (Damage :type Float%20%28single-precision%29) (DamageType :type Damage%20Type%20Object%20Reference) (InstigatedBy :type Controller%20Object%20Reference) (DamageCauser :type Actor%20Object%20Reference))
  (CallFunction|DamageServerNPC Damage))

(fn ConstructionScript)