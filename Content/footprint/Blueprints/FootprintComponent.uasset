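; Footprint component that plays surface footstep sounds and spawns decal prints under a character's feet.
; SpawnDecal traces down from a foot socket and passes the physical surface through SpawnServer and SpawnClient to SpawnFootprint.
; Sand, dirt, water and blood set a foot state, which hard surfaces turn into step-limited trails that fade via dynamic material parameters.
; Data tables supply decal materials by footwear and foot side; water itself leaves no print.
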(event Custom|SpawnClient
  (params (Location :type Vector) (Rotation :type Rotator) (Left :type Boolean) (Right :type Boolean) (SurfaceType :type EPhysicalSurface%20Enum :default "SurfaceType_Default"))
  ;[1 1 1] Line Trace to Ground
  (CallFunction|SpawnFootprint Location Rotation Left Right SurfaceType))

(event Custom|SpawnServer
  (params (Location :type Vector) (Rotation :type Rotator) (Left :type Boolean) (Right :type Boolean) (SurfaceType :type EPhysicalSurface%20Enum :default "SurfaceType_Default"))
  ;[1 1 1] Line Trace to Ground
  (CallFunction|SpawnClient Location Rotation Left Right SurfaceType))

(event EventSpawnDecal
  (params (SocketName :type Name :default "None") (Right :type Boolean) (Left :type Boolean))
  (bind _mesh (Variables|Default|GetMesh))
  (bind _mesh_2 (Variables|Default|GetMesh))
  (bind _returnvalue (Transformation|GetSocketLocation _mesh_2 SocketName))
  ;[1 1 1] Line Trace to Ground
  (bind (_outhit _returnvalue_2) (Collision|LineTraceByChannel (+ _returnvalue "0, 0,150.000000") (- _returnvalue "0, 0,50.000000") "TraceTypeQuery1" false 0 "None"))
  (if _returnvalue_2
    (Utilities|IsValid (.PhysMat (Collision|BreakHitResult _outhit))
      (:Is%20Valid
        (CallFunction|SpawnServer (.Location (Math|Transform|BreakTransform (Transformation|GetSocketTransform _mesh SocketName "RTS_World"))) (Math|Rotator|MakeRotator 0.0 (.Pitch (Math|Rotator|BreakRotator (Math|Conversions|RotationFromXVector (Math|Vector|NegateVector (.ImpactNormal (Collision|BreakHitResult _outhit)))))) (.Yaw (Math|Rotator|BreakRotator (Math|Conversions|RotationFromXVector (Math|Vector|GetForwardVector _mesh))))) Right Left (Variables|/Script/PhysicsCore.PhysicalMaterial|GetSurfaceType (.PhysMat (Collision|BreakHitResult _outhit))))))))

(fn SpawnFootprint
  (params (Location :type Vector) (Rotation :type Rotator) (Left :type Boolean) (Right :type Boolean) (SurfaceType :type EPhysicalSurface%20Enum :default "SurfaceType_Default"))
  (bind _currentfootwear (Variables|Default|GetCurrentFootwear))
  (bind _currentfootwear_2 (Variables|Default|GetCurrentFootwear))
  (bind _currentfootwear_3 (Variables|Default|GetCurrentFootwear))
  (bind _currentfootwear_4 (Variables|Default|GetCurrentFootwear))
  (bind _currentfootwear_5 (Variables|Default|GetCurrentFootwear))
  ;[1 1 1] Setting various Variables
  (Variables|Default|SetLocation Location)
  (Variables|Default|SetRotation Rotation)
  (Variables|Default|SetLeft Left)
  (Variables|Default|SetRight Right)
  ;[1 1 1] Determins on which SurfaceType a Decal should Spawn
  (switch Utilities|FlowControl|Switch|SwitchonEPhysicalSurface SurfaceType
    (:SurfaceType_Default
      ;[1 1 1] Switch Surface
      (Audio|PlaySoundatLocation "/Game/footprint/Sounds/Stone.Stone" (Variables|Default|GetLocation) "0, 0, 0" 0.2 (Math|Random|RandomFloatinRange 0.8 1.2) 0.0 0 0 0 :!label _label)
      ;[1 1 1] Check current FootState
      (switch Utilities|FlowControl|Switch|SwitchonEFootState (Variables|Default|GetFootState) :!label _label_2
        (:NewEnumerator1
          ;[1 1 1] Adjusting FootState or Check Database for the correct Material in this situation
          (if (>= (Variables|Default|GetCurrentMudSteps) (Variables|Default|GetMaxMudSteps))
            (Variables|Default|SetFootState "NewEnumerator0")
            (Variables|Default|SetCurrentMudSteps 0.0)
            (else
              (Math|Float|IncrementFloat (Variables|Default|GetCurrentMudSteps)
                (:%20%20
                  (bind _outrownames (DataTable|GetDataTableRowNames "/Game/footprint/Blueprints/Data/FootprintMudyDataTable.FootprintMudyDataTable"))
                  (for _array_element _outrownames
                    (bind _returnvalue (Utilities|GetDataTableRow "/Game/footprint/Blueprints/Data/FootprintMudyDataTable.FootprintMudyDataTable" _array_element)
                      (:then
                        (if (or (and (== (.Style (Utilities|Struct|BreakFootprintModifyStruct _returnvalue)) _currentfootwear) (Math|Boolean|Equal(Boolean) (.Right (Utilities|Struct|BreakFootprintModifyStruct _returnvalue)) (Variables|Default|GetRight))) (and (== (.Style (Utilities|Struct|BreakFootprintModifyStruct _returnvalue)) _currentfootwear) (Math|Boolean|Equal(Boolean) (.Left (Utilities|Struct|BreakFootprintModifyStruct _returnvalue)) (Variables|Default|GetLeft))))
                          ;[1 1 1] Spawn Footprint Actor with Correct Material Instance and Scalar Parameters
                          (bind _returnvalue_2 (Game|SpawnActorfromClass "/Game/footprint/Blueprints/Footprint_Actor.Footprint_Actor_C" (Math|Transform|MakeTransform (Variables|Default|GetLocation) (Variables|Default|GetRotation)) "AdjustIfPossibleButDontSpawnIfColliding" 0 0))
                          (Rendering|Components|Decal|SetDecalMaterial (Variables|/Game/footprint/Blueprints/Footprint_Actor.Footprint_Actor_C|GetFootprintDecal _returnvalue_2) (.MaterialInterface (Utilities|Struct|BreakFootprintModifyStruct _returnvalue)))
                          (bind _returnvalue_3 (Rendering|Material|CreateDynamicMaterialInstance (Variables|/Game/footprint/Blueprints/Footprint_Actor.Footprint_Actor_C|GetFootprintDecal _returnvalue_2) :!class /Script/Engine.DecalComponent))
                          (Rendering|Material|SetScalarParameterValue _returnvalue_3 "Flatness" (/ (Variables|Default|GetCurrentMudSteps) (Variables|Default|GetMaxMudSteps)) :!class /Script/Engine.MaterialInstanceDynamic)
                          (Rendering|Material|SetScalarParameterValue _returnvalue_3 "Opacityness" (- 1.0 (/ (Variables|Default|GetCurrentMudSteps) (Variables|Default|GetMaxMudSteps))) :!class /Script/Engine.MaterialInstanceDynamic))))))))))
        (:NewEnumerator2
          ;[1 1 1] Adjusting FootState or Check Database for the correct Material in this situation
          (if (>= (Variables|Default|GetCurrentSandSteps) (Variables|Default|GetMaxSandSteps))
            (Variables|Default|SetFootState "NewEnumerator0")
            (Variables|Default|SetCurrentSandSteps 0.0)
            (else
              (Math|Float|IncrementFloat (Variables|Default|GetCurrentSandSteps)
                (:%20%20
                  (bind _outrownames_2 (DataTable|GetDataTableRowNames "/Game/footprint/Blueprints/Data/FootprintSandyDataTable.FootprintSandyDataTable"))
                  (for _array_element_2 _outrownames_2
                    (bind _returnvalue_4 (Utilities|GetDataTableRow "/Game/footprint/Blueprints/Data/FootprintSandyDataTable.FootprintSandyDataTable" _array_element_2)
                      (:then
                        (if (or (and (== (.Style (Utilities|Struct|BreakFootprintModifyStruct _returnvalue_4)) _currentfootwear_2) (Math|Boolean|Equal(Boolean) (.Right (Utilities|Struct|BreakFootprintModifyStruct _returnvalue_4)) (Variables|Default|GetRight))) (and (== (.Style (Utilities|Struct|BreakFootprintModifyStruct _returnvalue_4)) _currentfootwear_2) (Math|Boolean|Equal(Boolean) (.Left (Utilities|Struct|BreakFootprintModifyStruct _returnvalue_4)) (Variables|Default|GetLeft))))
                          ;[1 1 1] Spawn Footprint Actor with Correct Material Instance and Scalar Parameters
                          (bind _returnvalue_5 (Game|SpawnActorfromClass "/Game/footprint/Blueprints/Footprint_Actor.Footprint_Actor_C" (Math|Transform|MakeTransform (Variables|Default|GetLocation) (Variables|Default|GetRotation)) "AdjustIfPossibleButDontSpawnIfColliding" 0 0))
                          (Rendering|Components|Decal|SetDecalMaterial (Variables|/Game/footprint/Blueprints/Footprint_Actor.Footprint_Actor_C|GetFootprintDecal _returnvalue_5) (.MaterialInterface (Utilities|Struct|BreakFootprintModifyStruct _returnvalue_4)))
                          (bind _returnvalue_6 (Rendering|Material|CreateDynamicMaterialInstance (Variables|/Game/footprint/Blueprints/Footprint_Actor.Footprint_Actor_C|GetFootprintDecal _returnvalue_5) :!class /Script/Engine.DecalComponent))
                          (Rendering|Material|SetScalarParameterValue _returnvalue_6 "Flatness" (/ (Variables|Default|GetCurrentSandSteps) (Variables|Default|GetMaxSandSteps)) :!class /Script/Engine.MaterialInstanceDynamic)
                          (Rendering|Material|SetScalarParameterValue _returnvalue_6 "Opacityness" (- 1.0 (/ (Variables|Default|GetCurrentSandSteps) (Variables|Default|GetMaxSandSteps))) :!class /Script/Engine.MaterialInstanceDynamic))))))))))
        (:NewEnumerator3
          ;[1 1 1] Adjusting FootState or Check Database for the correct Material in this situation
          (if (>= (Variables|Default|GetCurrentWetSteps) (Variables|Default|GetMaxWetSteps))
            (Variables|Default|SetFootState "NewEnumerator0")
            (Variables|Default|SetCurrentWetSteps 0.0)
            (else
              (Math|Float|IncrementFloat (Variables|Default|GetCurrentWetSteps)
                (:%20%20
                  (bind _outrownames_3 (DataTable|GetDataTableRowNames "/Game/footprint/Blueprints/Data/FootprintWetDataTable.FootprintWetDataTable"))
                  (for _array_element_3 _outrownames_3
                    (bind _returnvalue_7 (Utilities|GetDataTableRow "/Game/footprint/Blueprints/Data/FootprintWetDataTable.FootprintWetDataTable" _array_element_3)
                      (:then
                        (if (or (and (== (.Style (Utilities|Struct|BreakFootprintModifyStruct _returnvalue_7)) _currentfootwear_3) (Math|Boolean|Equal(Boolean) (.Right (Utilities|Struct|BreakFootprintModifyStruct _returnvalue_7)) (Variables|Default|GetRight))) (and (== (.Style (Utilities|Struct|BreakFootprintModifyStruct _returnvalue_7)) _currentfootwear_3) (Math|Boolean|Equal(Boolean) (.Left (Utilities|Struct|BreakFootprintModifyStruct _returnvalue_7)) (Variables|Default|GetLeft))))
                          ;[1 1 1] Spawn Footprint Actor with Correct Material Instance and Scalar Parameters
                          (bind _returnvalue_8 (Game|SpawnActorfromClass "/Game/footprint/Blueprints/Footprint_Actor.Footprint_Actor_C" (Math|Transform|MakeTransform (Variables|Default|GetLocation) (Variables|Default|GetRotation)) "AdjustIfPossibleButDontSpawnIfColliding" 0 0))
                          (Rendering|Components|Decal|SetDecalMaterial (Variables|/Game/footprint/Blueprints/Footprint_Actor.Footprint_Actor_C|GetFootprintDecal _returnvalue_8) (.MaterialInterface (Utilities|Struct|BreakFootprintModifyStruct _returnvalue_7)))
                          (bind _returnvalue_9 (Rendering|Material|CreateDynamicMaterialInstance (Variables|/Game/footprint/Blueprints/Footprint_Actor.Footprint_Actor_C|GetFootprintDecal _returnvalue_8) :!class /Script/Engine.DecalComponent))
                          (Rendering|Material|SetScalarParameterValue _returnvalue_9 "Flatness" (/ (Variables|Default|GetCurrentWetSteps) (Variables|Default|GetMaxWetSteps)) :!class /Script/Engine.MaterialInstanceDynamic)
                          (Rendering|Material|SetScalarParameterValue _returnvalue_9 "Opacityness" (- 1.0 (/ (Variables|Default|GetCurrentWetSteps) (Variables|Default|GetMaxWetSteps))) :!class /Script/Engine.MaterialInstanceDynamic))))))))))
        (:NewEnumerator4
          ;[1 1 1] Adjusting FootState or Check Database for the correct Material in this situation
          (if (>= (Variables|Default|GetCurrentBloodSteps) (Variables|Default|GetMaxBloodSteps))
            (Variables|Default|SetFootState "NewEnumerator0")
            (Variables|Default|SetCurrentBloodSteps 0.0)
            (else
              (Math|Float|IncrementFloat (Variables|Default|GetCurrentBloodSteps)
                (:%20%20
                  (bind _outrownames_4 (DataTable|GetDataTableRowNames "/Game/footprint/Blueprints/Data/FootprintBloodyDataTable.FootprintBloodyDataTable"))
                  (for _array_element_4 _outrownames_4
                    (bind _returnvalue_10 (Utilities|GetDataTableRow "/Game/footprint/Blueprints/Data/FootprintBloodyDataTable.FootprintBloodyDataTable" _array_element_4)
                      (:then
                        (if (or (and (== (.Style (Utilities|Struct|BreakFootprintModifyStruct _returnvalue_10)) _currentfootwear_5) (Math|Boolean|Equal(Boolean) (.Right (Utilities|Struct|BreakFootprintModifyStruct _returnvalue_10)) (Variables|Default|GetRight))) (and (== (.Style (Utilities|Struct|BreakFootprintModifyStruct _returnvalue_10)) _currentfootwear_5) (Math|Boolean|Equal(Boolean) (.Left (Utilities|Struct|BreakFootprintModifyStruct _returnvalue_10)) (Variables|Default|GetLeft))))
                          ;[1 1 1] Spawn Footprint Actor with Correct Material Instance and Scalar Parameters
                          (bind _returnvalue_11 (Game|SpawnActorfromClass "/Game/footprint/Blueprints/Footprint_Actor.Footprint_Actor_C" (Math|Transform|MakeTransform (Variables|Default|GetLocation) (Variables|Default|GetRotation)) "AdjustIfPossibleButDontSpawnIfColliding" 0 0))
                          (Rendering|Components|Decal|SetDecalMaterial (Variables|/Game/footprint/Blueprints/Footprint_Actor.Footprint_Actor_C|GetFootprintDecal _returnvalue_11) (.MaterialInterface (Utilities|Struct|BreakFootprintModifyStruct _returnvalue_10)))
                          (bind _returnvalue_12 (Rendering|Material|CreateDynamicMaterialInstance (Variables|/Game/footprint/Blueprints/Footprint_Actor.Footprint_Actor_C|GetFootprintDecal _returnvalue_11) :!class /Script/Engine.DecalComponent))
                          (Rendering|Material|SetScalarParameterValue _returnvalue_12 "Flatness" (/ (Variables|Default|GetCurrentBloodSteps) (Variables|Default|GetMaxBloodSteps)) :!class /Script/Engine.MaterialInstanceDynamic)
                          (Rendering|Material|SetScalarParameterValue _returnvalue_12 "Opacityness" (- 1.0 (/ (Variables|Default|GetCurrentBloodSteps) (Variables|Default|GetMaxBloodSteps))) :!class /Script/Engine.MaterialInstanceDynamic))))))))))))
    (:SurfaceType1
      (Audio|PlaySoundatLocation "/Game/footprint/Sounds/Sand.Sand" (Variables|Default|GetLocation) "0, 0, 0" 0.5 (Math|Random|RandomFloatinRange 0.8 1.2) 0.0 0 0 0)
      ;[1 1 1] Setting State Parameters and Current Step
      (Variables|Default|SetFootState "NewEnumerator2")
      (Variables|Default|SetCurrentSandSteps 0.0)
      ;[1 1 1] Check Database for the correct Material in this situation
      (bind _outrownames_5 (DataTable|GetDataTableRowNames "/Game/footprint/Blueprints/Data/FootprintDataTable.FootprintDataTable" :!label _label_3))
      (for _array_element_5 _outrownames_5
        (bind _returnvalue_13 (Utilities|GetDataTableRow "/Game/footprint/Blueprints/Data/FootprintDataTable.FootprintDataTable" _array_element_5)
          (:then
            (if (or (and (== (.Style (Utilities|Struct|BreakFootprintModifyStruct _returnvalue_13)) _currentfootwear_4) (Math|Boolean|Equal(Boolean) (.Right (Utilities|Struct|BreakFootprintModifyStruct _returnvalue_13)) (Variables|Default|GetRight))) (and (== (.Style (Utilities|Struct|BreakFootprintModifyStruct _returnvalue_13)) _currentfootwear_4) (Math|Boolean|Equal(Boolean) (.Left (Utilities|Struct|BreakFootprintModifyStruct _returnvalue_13)) (Variables|Default|GetLeft))))
              ;[1 1 1] Spawn Footprint Actor with correct Material
              (bind _returnvalue_14 (Game|SpawnActorfromClass "/Game/footprint/Blueprints/Footprint_Actor.Footprint_Actor_C" (Math|Transform|MakeTransform (Variables|Default|GetLocation) (Variables|Default|GetRotation)) "AdjustIfPossibleButDontSpawnIfColliding" 0 0))
              (Rendering|Components|Decal|SetDecalMaterial (Variables|/Game/footprint/Blueprints/Footprint_Actor.Footprint_Actor_C|GetFootprintDecal _returnvalue_14) (.MaterialInterface (Utilities|Struct|BreakFootprintModifyStruct _returnvalue_13))))))))
    (:SurfaceType2
      (goto _label))
    (:SurfaceType3
      (Audio|PlaySoundatLocation "/Game/footprint/Sounds/Mud.Mud" (Variables|Default|GetLocation) "0, 0, 0" 0.3 (Math|Random|RandomFloatinRange 0.8 1.2) 0.0 0 0 0)
      (Variables|Default|SetFootState "NewEnumerator1")
      (Variables|Default|SetCurrentMudSteps 0.0)
      (goto _label_3))
    (:SurfaceType4
      (Audio|PlaySoundatLocation "/Game/footprint/Sounds/Water.Water" (Variables|Default|GetLocation) "0, 0, 0" 0.2 (Math|Random|RandomFloatinRange 0.8 1.2) 0.0 0 0 0)
      ;[1 1 1] Not Spawning Any Footprints for Water
      (Variables|Default|SetFootState "NewEnumerator3")
      (Variables|Default|SetCurrentWetSteps 0.0))
    (:SurfaceType5
      (Audio|PlaySoundatLocation "/Game/footprint/Sounds/Blood.Blood" (Variables|Default|GetLocation) "0, 0, 0" 0.2 (Math|Random|RandomFloatinRange 0.8 1.2) 0.0 0 0 0)
      ;[1 1 1] Special Blood Treatment
      (Variables|Default|SetFootState "NewEnumerator4")
      (Variables|Default|SetCurrentBloodSteps 0.0)
      (goto _label_2))))